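; Player controller for a time attack race that drives the HUD and starts the race clock.
; On BeginPlay it creates the HUD with a splash screen and caches the TimeAttackGameState.
; The first left click runs a delayed countdown, swaps to the game HUD, then flags the race start and stamps race and lap times in the GameState.
; Tick hides the gold, silver and bronze target times as the current time passes each threshold.
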(event `self.ReceiveBeginPlay`
  ;[1 1 1] Set the HUD
  (bind _returnvalue (`|CreateWidget` "/Game/UI/HUD.HUD_C"))
  (bind _output_get (set `self.HUDReferece` _returnvalue))
  (`UserWidget.AddToViewport` _output_get 0)
  (set `/Game/UI/HUD.SplashScreenVisible` "Visible" (`self.HUDReferece`))
  ;[1 1 1] Get the GameState reference
  (bind _astime_attack_game_state (cast `TimeAttackGameState` (`GameplayStatics.GetGameState`)))
  (set `self.GameStateReference` _astime_attack_game_state))

(event `Key|LeftMouseButton`
  (params (Key :type "Key Structure" :default "AnyKey"))
  (bind _returnvalue (`GameplayStatics.GetTimeSeconds`))
  (bind _gamestatereference (`self.GameStateReference`))
  (bind _hudreferece (`self.HUDReferece`))
  (bind _hudreferece_2 (`self.HUDReferece`))
  ;[1 1 1] Manage the HUD before the start
  (:`Pressed`
    (`/Engine/EditorBlueprintResources/StandardMacros.DoOnce` false
      (:`Completed`
        (set `/Game/UI/HUD.SplashScreenVisible` "Hidden" _hudreferece)
        (set `/Game/UI/HUD.CountDownVisible` "Visible" _hudreferece)
        (`KismetSystemLibrary.Delay` 1.5)
        (set `self.ReadyText` "2")
        (`KismetSystemLibrary.Delay` 1.0)
        (set `self.ReadyText` "1")
        (`KismetSystemLibrary.Delay` 1.0)
        (set `self.ReadyText` "GO!")
        (`KismetSystemLibrary.Delay` 1.0)
        (set `/Game/UI/HUD.CountDownVisible` "Hidden" _hudreferece_2)
        (set `/Game/UI/HUD.GameHUDVisible` "Visible" _hudreferece_2)
        ;[1 1 1] Set the time at the start of the race
        (`TimeAttackGameState.SetRaceStart` _gamestatereference true)
        (`TimeAttackGameState.SetStartTimeRace` _gamestatereference _returnvalue)
        (`TimeAttackGameState.SetStartTimeLap` _gamestatereference _returnvalue)))))

(event `self.ReceiveTick`
  (params (DeltaSeconds :type "Float (single-precision)"))
  (bind _hudreferece (`self.HUDReferece`))
  (bind _returnvalue (`TimeAttackGameState.GetCurrentTime` (`self.GameStateReference`)))
  ;[1 1 1] Manage the visibility of Gold, Silver and Bronze times in the HUD
  (if (> _returnvalue 60.0)
    (set `/Game/UI/HUD.GoldTimeVisible` "Hidden" _hudreferece)
    (if (> _returnvalue 90.0)
      (set `/Game/UI/HUD.SilverTimeVisible` "Hidden" _hudreferece)
      (if (> _returnvalue 120.0)
        (set `/Game/UI/HUD.BronzeTimeVisible` "Hidden" _hudreferece)))))

(fn `UserConstructionScript`)